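; An openable door actor that swings open and closed through the OpenDoor events OnOpen and OnClose.
; It stores its rotation at BeginPlay, and the DoorSwing timeline adds an animated yaw to it each update.
; Opening plays the timeline forward and closing reverses it.
; The open-door sound and a delay node are present but unconnected, so the door is silent.
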(event OnOpen(OpenDoor)
  (bind _opendoor (Timeline|DoorSwing Play)
    (:Update
      (Transformation|SetActorRotation (Math|Rotator|CombineRotators (Math|Rotator|MakeRotator 0.0 0.0 _opendoor) (Variables|Default|GetInitialRotation))))))

(event OnClose(OpenDoor)
  (bind _opendoor (Timeline|DoorSwing Reverse)
    (:Update
      (Transformation|SetActorRotation (Math|Rotator|CombineRotators (Math|Rotator|MakeRotator 0.0 0.0 _opendoor) (Variables|Default|GetInitialRotation))))))

(event EventBeginPlay
  (Variables|Default|SetInitialRotation (Transformation|GetActorRotation)))

(fn ConstructionScript)